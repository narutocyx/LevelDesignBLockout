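; Door Blueprint that handles interaction and unlocking, with a text render prompt showing lock status.
; Interact shows the locked text while locked; otherwise a FlipFlop alternates OpenDoor and CloseDoor, hiding the prompt on open and showing it on close.
; Unlock clears the lock flag and switches the prompt to the unlocked text.
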(event `/Game/Blueprints/FirstPersonTemplate/BPI_Interaction.Interact`
  (bind _textrender_ui (`self.TextRender_UI`))
  (if (`self.IsLocked`)
    (`TextRenderComponent.K2_SetText` (`self.TextRender_UI`) (`self.LockedText`))
    (else
      (`/Engine/EditorBlueprintResources/StandardMacros.FlipFlop`
        (:`A`
          (`self.OpenDoor`)
          (`SceneComponent.SetHiddenInGame` _textrender_ui true false))
        (:`B`
          (`self.CloseDoor`)
          (`SceneComponent.SetHiddenInGame` _textrender_ui false false))))))

(event `/Game/Blueprints/FirstPersonTemplate/BPI_Interaction.Unlock`
  (set `self.IsLocked` false)
  (`TextRenderComponent.K2_SetText` (`self.TextRender_UI`) (`self.UnlockedText`)))

(fn `UserConstructionScript`
  (`parent.UserConstructionScript`))
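; Parent Blueprint for a hinged door that swings open and closed and shows a text prompt when approached.
; OpenDoor and CloseDoor play and reverse a timeline that lerps the door's relative yaw.
; When the timeline finishes, its direction sets IsOpen and the text is hidden either way.
; Sphere overlaps toggle the text only while IsOpen is false, without filtering the overlapping actor.
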(event `OpenDoor`
  (bind _textrender_ui (`self.TextRender_UI`))
  ;[1 1 1] Door Animation
  (bind (_direction _door_alpha) (`Timeline|DoorAnimation` :!label _label)
    (:`Update`
      (`SceneComponent.K2_SetRelativeRotation` (`self.Door`) (`KismetMathLibrary.RLerp` (struct) (struct :`Yaw` -110.0) _door_alpha true) false false))
    (:`Finished`
      (switch `ETimelineDirection` _direction
        (:`Forward`
          (set `self.IsOpen` true)
          (`SceneComponent.SetHiddenInGame` _textrender_ui true false))
        (:`Backward`
          (set `self.IsOpen` false)
          (`SceneComponent.SetHiddenInGame` _textrender_ui true false))))))

(event `CloseDoor`
  ;[1 1 1] Door Animation
  (goto _label :!via `Reverse`))

(event `self.Sphere.OnComponentBeginOverlap`
  (params (OverlappedComponent :type "PrimitiveComponent Object Reference") (OtherActor :type "Actor Object Reference") (OtherComp :type "PrimitiveComponent Object Reference") (OtherBodyIndex :type Integer) (bFromSweep :type Boolean) (SweepResult :type "HitResult Structure (by ref)"))
  ;[1 1 1] UI
  (if (not (`self.IsOpen`))
    (`SceneComponent.SetHiddenInGame` (`self.TextRender_UI`) false false)))

(event `self.Sphere.OnComponentEndOverlap`
  (params (OverlappedComponent :type "PrimitiveComponent Object Reference") (OtherActor :type "Actor Object Reference") (OtherComp :type "PrimitiveComponent Object Reference") (OtherBodyIndex :type Integer))
  ;[1 1 1] UI
  (if (not (`self.IsOpen`))
    (`SceneComponent.SetHiddenInGame` (`self.TextRender_UI`) true false)))

(fn `UserConstructionScript`)
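; BPC_Switch is a one-shot interactable switch that can start locked, built on a parent interaction Blueprint.
; Interacting while locked shows the locked text; otherwise a DoOnce plays a timeline that lowers the mesh slightly, then fires OnInteractionComplete.
; The construction script colors the mesh red or green from IsLocked, and Unlock clears the lock and turns it green.
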(event `self.StartEventsOnInteract`
  (if (`self.IsLocked`)
    (`TextRenderComponent.K2_SetText` (`self.InteractUI`) (`self.LockedText`))
    (else
      (`/Engine/EditorBlueprintResources/StandardMacros.DoOnce` false
        (:`Completed`
          (bind (_direction _driver) (`Timeline|Timeline_0`)
            (:`Update`
              (`SceneComponent.K2_SetRelativeLocation` (`self.StaticMesh`) (`KismetMathLibrary.VLerp` (0.0 0.0 0.0) (0.0 0.0 -5.0) _driver) false false))
            (:`Finished`
              (switch `ETimelineDirection` _direction
                (:`Forward`
                  (`self.OnInteractionComplete`))))))))))

(event `/Game/Blueprints/FirstPersonTemplate/BPI_Interaction.Unlock`
  (set `self.IsLocked` false)
  (`PrimitiveComponent.SetMaterial` (`self.StaticMesh`) 0 "/Game/Materials/MI_LDGrid_Local_Green.MI_LDGrid_Local_Green"))

(fn `UserConstructionScript`
  (bind _staticmesh (`self.StaticMesh`))
  (`parent.UserConstructionScript`)
  (if (`self.IsLocked`)
    (`PrimitiveComponent.SetMaterial` _staticmesh 0 "/Game/Materials/MI_LDGrid_Local_Red.MI_LDGrid_Local_Red")
    (else
      (`PrimitiveComponent.SetMaterial` _staticmesh 0 "/Game/Materials/MI_LDGrid_Local_Green.MI_LDGrid_Local_Green"))))
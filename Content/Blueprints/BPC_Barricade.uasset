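; BPC_Barricade is an interactable barricade that collapses when interacted with.
; On the interact event, its four static meshes start simulating physics and their rigid bodies are woken, so the pieces can fall.
; After a short delay it disables collision on all four meshes and calls OnInteractionComplete to signal the interaction has finished.
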(event `self.StartEventsOnInteract`
  (bind _staticmesh1 (`self.StaticMesh1`))
  (`PrimitiveComponent.SetSimulatePhysics` _staticmesh1 true)
  (`PrimitiveComponent.SetSimulatePhysics` (`self.StaticMesh2`) true)
  (`PrimitiveComponent.SetSimulatePhysics` (`self.StaticMesh3`) true)
  (`PrimitiveComponent.SetSimulatePhysics` (`self.StaticMesh`) true)
  (`PrimitiveComponent.WakeAllRigidBodies` _staticmesh1)
  (`PrimitiveComponent.WakeAllRigidBodies` (`self.StaticMesh2`))
  (`PrimitiveComponent.WakeAllRigidBodies` (`self.StaticMesh3`))
  (`PrimitiveComponent.WakeAllRigidBodies` (`self.StaticMesh`))
  (`KismetSystemLibrary.Delay` 2.0)
  (`PrimitiveComponent.SetCollisionEnabled` (`self.StaticMesh`) "NoCollision")
  (`PrimitiveComponent.SetCollisionEnabled` (`self.StaticMesh1`) "NoCollision")
  (`PrimitiveComponent.SetCollisionEnabled` (`self.StaticMesh2`) "NoCollision")
  (`PrimitiveComponent.SetCollisionEnabled` (`self.StaticMesh3`) "NoCollision")
  (`self.OnInteractionComplete`))

(fn `UserConstructionScript`
  (`parent.UserConstructionScript`))
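; BPC_GearMachine is a child Blueprint for an interactable gear machine that reveals a mesh when used unlocked.
; It implements StartEventsonInteract: while IsLocked it shows LockedText on InteractUI.
; Otherwise it unhides StaticMesh, hides InteractUI and calls OnInteractionComplete.
; The construction script only runs the parent's version.
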(event `self.StartEventsOnInteract`
  (if (`self.IsLocked`)
    (`TextRenderComponent.K2_SetText` (`self.InteractUI`) (`self.LockedText`))
    (else
      (`SceneComponent.SetHiddenInGame` (`self.StaticMesh`) false false)
      (`SceneComponent.SetHiddenInGame` (`self.InteractUI`) true false)
      (`self.OnInteractionComplete`))))

(fn `UserConstructionScript`
  (`parent.UserConstructionScript`))